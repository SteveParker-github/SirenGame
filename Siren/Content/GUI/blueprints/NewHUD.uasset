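; HUD Blueprint that procedurally generates crew characters and prepares hiring options for the game's GUI.
; Creators per type (captain, rower, archer, soldier) roll names from a DataTable and random stats, then derive a value from both.
; The construction script builds a hireable pool of non-captains, formats it into per-type text and fills three option variables.
; CreateCrew, not called here, assembles a crew from requested counts with a fixed player or random captain.
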(event EventBeginPlay)

(event Collision|EventActorBeginOverlap
  (params (OtherActor :type Actor%20Object%20Reference)))

(event EventTick
  (params (DeltaSeconds :type Float%20%28single-precision%29)))

(fn ConstructionScript
  (CallFunction|CreateHireable))

(fn RoundFloat
  (params (FloatIN :type Float%20%28single-precision%29))
  (return (/ (Math|Conversions|ToFloat(Integer) (Math|Float|Round (* 100 FloatIN))) 1e+02)))

(fn CreateName
  (Utilities|FlowControl|Sequence
    (:then_0
      (bind _returnvalue (Class|DataTableFunctionLibrary|GetDataTableColumnasString "/Game/Characters/Names.Names" "FirstName"))
      (bind _output_get (Variables|Default|SetFirstNames _returnvalue))
      (Variables|Default|SetFirstName (.OutItem (Utilities|Array|Random _output_get))))
    (:then_1
      (bind _returnvalue_2 (Class|DataTableFunctionLibrary|GetDataTableColumnasString "/Game/Characters/Names.Names" "LastName"))
      (bind _output_get_2 (Variables|Default|SetLastNames _returnvalue_2))
      (Variables|Default|SetLastName (.OutItem (Utilities|Array|Random _output_get_2))))
    (:then_2
      (bind _output_get_3 (Variables|Default|Setname (Utilities|Struct|MakeName (Variables|Default|GetFirstName) (Variables|Default|GetLastName))))
      (return _output_get_3))))

(fn SetRegen
  (bind _floatout (CallFunction|RoundFloat (Math|Random|RandomFloatinRange 0.1 2.0)))
  (bind _output_get (Variables|Default|Setregen _floatout))
  (return _output_get))

(fn SetHealth
  (params (Max :type Integer))
  (bind _output_get (Variables|Default|Sethealth (Math|Random|RandomIntegerinRange 10 Max)))
  (return _output_get))

(fn SetValue
  (params (CharacterType :type CharacterType%20Enum :default "NewEnumerator0") (HealthIN :type Integer) (StaminaIN :type Integer) (RegenIN :type Float%20%28single-precision%29))
  (Variables|Default|SetCharacterType CharacterType)
  (Variables|Default|SetHealth HealthIN)
  (Variables|Default|SetStamina StaminaIN)
  (Variables|Default|SetRegen RegenIN)
  (Utilities|FlowControl|Sequence
    (:then_0
      (switch Utilities|FlowControl|Switch|SwitchonCharacterType (Variables|Default|GetCharacterType)
        (:NewEnumerator0
          (Variables|Default|SetValue 20))
        (:NewEnumerator1
          (Variables|Default|SetValue 8))
        (:NewEnumerator2
          (Variables|Default|SetValue 6))
        (:NewEnumerator3
          (Variables|Default|SetValue 10))))
    (:then_1
      (LocalVariables|SetHealthStaminaValue (+ (* (Variables|Default|GetHealth) (Variables|Default|GetValue)) (* (Variables|Default|GetStamina) (Variables|Default|GetValue)))))
    (:then_2
      (bind _floatout (CallFunction|RoundFloat (* (Variables|Default|GetValue) (Variables|Default|GetRegen))))
      (bind _floatout_2 (CallFunction|RoundFloat (+ _floatout (Math|Conversions|ToFloat(Integer) (LocalVariables|GetHealthStaminaValue)))))
      (bind _output_get (Variables|Default|SetValue (Math|Float|Truncate _floatout_2)))
      (return _output_get))))

(fn SetStamina
  (params (Max :type Integer))
  (bind _output_get (Variables|Default|Setstamina (Math|Random|RandomIntegerinRange 10 Max)))
  (return _output_get))

(fn CreateRower
  (params (name :type Name%20Structure))
  (Variables|Default|Setname name)
  (Variables|Default|SetCharacterType "NewEnumerator1")
  (Utilities|FlowControl|Sequence
    (:then_0
      (bind _health (CallFunction|SetHealth 50))
      (Variables|Default|Sethealth _health))
    (:then_1
      (bind _stamina (CallFunction|SetStamina 100))
      (Variables|Default|Setstamina _stamina))
    (:then_2
      (bind _regen (CallFunction|SetRegen))
      (Variables|Default|Setregen _regen))
    (:then_3
      (bind _returnvalue (CallFunction|SetValue (Variables|Default|GetCharacterType) (Variables|Default|Gethealth) (Variables|Default|Getstamina) (Variables|Default|Getregen)))
      (Variables|Default|Setvalue _returnvalue))
    (:then_4
      (bind _output_get (Variables|Default|SetCharacter (Utilities|Struct|MakeCharacter (Variables|Default|GetCharacterType) (Variables|Default|Getname) (Variables|Default|Gethealth) (Variables|Default|Getstamina) (Variables|Default|Getregen) (Variables|Default|Getvalue))))
      (return _output_get))))

(fn CreateSoldier
  (params (name :type Name%20Structure))
  (Variables|Default|Setname name)
  (Variables|Default|SetCharacterType "NewEnumerator3")
  (Utilities|FlowControl|Sequence
    (:then_0
      (bind _health (CallFunction|SetHealth 100))
      (Variables|Default|Sethealth _health))
    (:then_1
      (bind _stamina (CallFunction|SetStamina 50))
      (Variables|Default|Setstamina _stamina))
    (:then_2
      (bind _regen (CallFunction|SetRegen))
      (Variables|Default|Setregen _regen))
    (:then_3
      (bind _returnvalue (CallFunction|SetValue (Variables|Default|GetCharacterType) (Variables|Default|Gethealth) (Variables|Default|Getstamina) (Variables|Default|Getregen)))
      (Variables|Default|Setvalue _returnvalue))
    (:then_4
      (bind _output_get (Variables|Default|SetCharacter (Utilities|Struct|MakeCharacter (Variables|Default|GetCharacterType) (Variables|Default|Getname) (Variables|Default|Gethealth) (Variables|Default|Getstamina) (Variables|Default|Getregen) (Variables|Default|Getvalue))))
      (return _output_get))))

(fn CreateCaptain
  (params (name :type Name%20Structure))
  (Variables|Default|Setname name)
  (Variables|Default|SetCharacterType "NewEnumerator0")
  (Utilities|FlowControl|Sequence
    (:then_0
      (bind _health (CallFunction|SetHealth 100))
      (Variables|Default|Sethealth _health))
    (:then_1
      (bind _stamina (CallFunction|SetStamina 100))
      (Variables|Default|Setstamina _stamina))
    (:then_2
      (bind _regen (CallFunction|SetRegen))
      (Variables|Default|Setregen _regen))
    (:then_3
      (bind _returnvalue (CallFunction|SetValue (Variables|Default|GetCharacterType) (Variables|Default|Gethealth) (Variables|Default|Getstamina) (Variables|Default|Getregen)))
      (Variables|Default|Setvalue _returnvalue))
    (:then_4
      (bind _output_get (Variables|Default|SetCharacter (Utilities|Struct|MakeCharacter (Variables|Default|GetCharacterType) (Variables|Default|Getname) (Variables|Default|Gethealth) (Variables|Default|Getstamina) (Variables|Default|Getregen) (Variables|Default|Getvalue))))
      (return _output_get))))

(fn CreateArcher
  (params (name :type Name%20Structure))
  (Variables|Default|Setname name)
  (Variables|Default|SetCharacterType "NewEnumerator2")
  (Utilities|FlowControl|Sequence
    (:then_0
      (bind _health (CallFunction|SetHealth 75))
      (Variables|Default|Sethealth _health))
    (:then_1
      (bind _stamina (CallFunction|SetStamina 75))
      (Variables|Default|Setstamina _stamina))
    (:then_2
      (bind _regen (CallFunction|SetRegen))
      (Variables|Default|Setregen _regen))
    (:then_3
      (bind _returnvalue (CallFunction|SetValue (Variables|Default|GetCharacterType) (Variables|Default|Gethealth) (Variables|Default|Getstamina) (Variables|Default|Getregen)))
      (Variables|Default|Setvalue _returnvalue))
    (:then_4
      (bind _output_get (Variables|Default|SetCharacter (Utilities|Struct|MakeCharacter (Variables|Default|GetCharacterType) (Variables|Default|Getname) (Variables|Default|Gethealth) (Variables|Default|Getstamina) (Variables|Default|Getregen) (Variables|Default|Getvalue))))
      (return _output_get))))

(fn CreatePlayer
  (Utilities|FlowControl|Sequence
    (:then_0
      (Variables|Default|Setname (Utilities|Struct|MakeName "Lakovos")))
    (:then_1
      (Variables|Default|SetCharacterType "NewEnumerator0"))
    (:then_2
      (Variables|Default|Sethealth 100))
    (:then_3
      (Variables|Default|Setstamina 100))
    (:then_4
      (Variables|Default|Setregen 1.0))
    (:then_5
      (Variables|Default|Setvalue 0))
    (:then_6
      (bind _output_get (Variables|Default|SetCharacter (Utilities|Struct|MakeCharacter (Variables|Default|GetCharacterType) (Variables|Default|Getname) (Variables|Default|Gethealth) (Variables|Default|Getstamina) (Variables|Default|Getregen) (Variables|Default|Getvalue))))
      (return _output_get))))

(fn CreateCharacter
  (params (CharacterType :type CharacterType%20Enum :default "NewEnumerator0"))
  (Variables|Default|SetCharacterType CharacterType)
  (Utilities|FlowControl|Sequence
    (:then_0
      ;[1 1 1] Setting Name
      (bind _name (CallFunction|CreateName))
      (Variables|Default|Setname _name))
    (:then_1
      (switch Utilities|FlowControl|Switch|SwitchonCharacterType (Variables|Default|GetCharacterType)
        (:NewEnumerator0
          (bind _character (CallFunction|CreateCaptain (Variables|Default|Getname)))
          (Variables|Default|SetCharacter _character))
        (:NewEnumerator1
          (bind _character_2 (CallFunction|CreateRower (Variables|Default|Getname)))
          (Variables|Default|SetCharacter _character_2))
        (:NewEnumerator2
          (bind _character_3 (CallFunction|CreateArcher (Variables|Default|Getname)))
          (Variables|Default|SetCharacter _character_3))
        (:NewEnumerator3
          (bind _character_4 (CallFunction|CreateSoldier (Variables|Default|Getname)))
          (Variables|Default|SetCharacter _character_4))))
    (:then_2
      (return (Variables|Default|GetCharacter)))))

(fn CreateCrew
  (params (CrewValues :type Create%20Crew%20Structure))
  (LocalVariables|SetCrewCount CrewValues)
  (Utilities|FlowControl|Sequence
    (:then_0
      (bind _enumvalue (|ForEachCharacterType)
        (:LoopBody
          (bind _output_get (LocalVariables|SetType _enumvalue))
          (if (Utilities|Enum|NotEqual(Enum) _output_get "NewEnumerator0")
            (switch Utilities|FlowControl|Switch|SwitchonCharacterType (LocalVariables|GetType)
              (:NewEnumerator1
                (for _index (range 0 (- (.num_rowers (Variables|Default|GetSetCrew)) 1))
                  (bind _character (CallFunction|CreateCharacter (LocalVariables|GetType)))
                  (LocalVariables|SetChar _character)
                  (switch Utilities|FlowControl|Switch|SwitchonCharacterType (LocalVariables|GetType)
                    (:NewEnumerator1
                      (Utilities|Array|Insert (LocalVariables|GetRowers) (LocalVariables|GetChar)))
                    (:NewEnumerator2
                      (Utilities|Array|Insert (LocalVariables|GetArchers) (LocalVariables|GetChar)))
                    (:NewEnumerator3
                      (Utilities|Array|Insert (LocalVariables|GetSoldiers) (LocalVariables|GetChar))))))
              (:NewEnumerator2
                (for _index_2 (range 0 (- 0 (.num_archers (Variables|Default|GetSetCrew))))
                  (bind _character_2 (CallFunction|CreateCharacter (LocalVariables|GetType)))
                  (LocalVariables|SetChar _character_2)
                  (switch Utilities|FlowControl|Switch|SwitchonCharacterType (LocalVariables|GetType)
                    (:NewEnumerator1
                      (Utilities|Array|Insert (LocalVariables|GetRowers) (LocalVariables|GetChar)))
                    (:NewEnumerator2
                      (Utilities|Array|Insert (LocalVariables|GetArchers) (LocalVariables|GetChar)))
                    (:NewEnumerator3
                      (Utilities|Array|Insert (LocalVariables|GetSoldiers) (LocalVariables|GetChar))))))
              (:NewEnumerator3
                (for _index_3 (range 0 (- (.num_soldiers (Variables|Default|GetSetCrew)) 1))
                  (bind _character_3 (CallFunction|CreateCharacter (LocalVariables|GetType)))
                  (LocalVariables|SetChar _character_3)
                  (switch Utilities|FlowControl|Switch|SwitchonCharacterType (LocalVariables|GetType)
                    (:NewEnumerator1
                      (Utilities|Array|Insert (LocalVariables|GetRowers) (LocalVariables|GetChar)))
                    (:NewEnumerator2
                      (Utilities|Array|Insert (LocalVariables|GetArchers) (LocalVariables|GetChar)))
                    (:NewEnumerator3
                      (Utilities|Array|Insert (LocalVariables|GetSoldiers) (LocalVariables|GetChar)))))))
            (elif (.player (Variables|Default|GetSetCrew))
              (bind _character_4 (CallFunction|CreatePlayer))
              (LocalVariables|SetCaptain _character_4)
              (else
                (bind _character_5 (CallFunction|CreateCharacter (LocalVariables|GetType)))
                (LocalVariables|SetCaptain _character_5)))))))
    (:then_1
      (bind _output_get_2 (LocalVariables|SetCrew (Utilities|Struct|MakeCrew (LocalVariables|GetCaptain) (LocalVariables|GetArchers) (LocalVariables|GetRowers) (LocalVariables|GetSoldiers))))
      (return _output_get_2))))

(fn SetHireable
  (Utilities|FlowControl|Sequence
    (:then_0
      (bind _enumvalue (|ForEachCharacterType)
        (:LoopBody
          (bind _output_get (Variables|Default|SetCharacterType _enumvalue))
          (if (Utilities|Enum|NotEqual(Enum) _output_get "NewEnumerator0")
            (for _index (range 0 4)
              (bind _character (CallFunction|CreateCharacter (Variables|Default|GetCharacterType)))
              (Utilities|Array|Insert (Variables|Default|GetHireable) _character))))))
    (:then_1
      (return (Variables|Default|GetHireable)))))

(fn SetHireableStr
  (params (Array :type Array%20of%20Character%20Structures))
  (for _array_element Array
    (Variables|Default|SetCharacterType (.Type (Utilities|Struct|BreakCharacter _array_element)))
    (Variables|Default|SetHirebleStr (Utilities|Text|ToText(String) (Utilities|String|Append (.FirstName (Utilities|Struct|BreakName (.Name (Utilities|Struct|BreakCharacter _array_element)))) " " (.LastName (Utilities|Struct|BreakName (.Name (Utilities|Struct|BreakCharacter _array_element)))) " 
" "Health: " (Utilities|String|ToString(Integer) (.Health (Utilities|Struct|BreakCharacter _array_element))) " Stamina: " (Utilities|String|ToString(Integer) (.Stamina (Utilities|Struct|BreakCharacter _array_element))) " 
" "Regen Speed:" (Utilities|String|ToString(Float) (.RegenSpeed (Utilities|Struct|BreakCharacter _array_element))) " Value: $" (Utilities|String|ToString(Integer) (.Value (Utilities|Struct|BreakCharacter _array_element))))))
    (switch Utilities|FlowControl|Switch|SwitchonCharacterType (Variables|Default|GetCharacterType)
      (:NewEnumerator1
        (Utilities|Array|Insert (Variables|Default|GetHireable_Rower) (Variables|Default|GetHirebleStr)))
      (:NewEnumerator2
        (Utilities|Array|Insert (Variables|Default|GetHireable_Archer) (Variables|Default|GetHirebleStr)))
      (:NewEnumerator3
        (Utilities|Array|Insert (Variables|Default|GetHireable_Soldier) (Variables|Default|GetHirebleStr))))))

(fn SetHireableTextBlocks
  (Utilities|FlowControl|Sequence
    (:then_0
      (Variables|Default|SetOption1 (Utilities|Array|Get(acopy) (Variables|Default|GetHireable_Archer))))
    (:then_1
      (Variables|Default|SetOption2 (Utilities|Array|Get(acopy) (Variables|Default|GetHireable_Soldier))))
    (:then_2
      (Variables|Default|SetOption3 (Utilities|Array|Get(acopy) (Variables|Default|GetHireable_Rower))))))

(fn CreateHireable
  (bind _hireable (CallFunction|SetHireable))
  (bind _output_get (Variables|Default|SetHireable _hireable))
  (CallFunction|SetHireableStr _output_get)
  (CallFunction|SetHireableTextBlocks))