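; BP_DockInfoIcon is a spinning info icon, apparently for the dock, that shows a message to the first-person character.
; Tick spins the actor at a constant yaw rate while the player pawn is BP_FPCharacter; otherwise, if the widget is valid, it removes it and hides the mesh.
; When that character enters TriggerBox, it creates a BP_MessageWidget and hides the mesh; leaving removes the widget and shows the mesh again.
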(event OnComponentBeginOverlap(TriggerBox)
  (params (OverlappedComponent :type Primitive%20Component%20Object%20Reference) (OtherActor :type Actor%20Object%20Reference) (OtherComp :type Primitive%20Component%20Object%20Reference) (OtherBodyIndex :type Integer) (bFromSweep :type Boolean) (SweepResult :type Hit%20Result%20Structure%20%28by%20ref%29))
  (Utilities|Casting|CastToBP_FPCharacter OtherActor)
  (bind _returnvalue (UserInterface|CreateWidget "/Game/UI/BP_MessageWidget.BP_MessageWidget_C" (Game|GetPlayerController 0)))
  (bind _output_get (Variables|Default|SetMessageWidget _returnvalue))
  (UserInterface|Viewport|AddtoViewport _output_get 0)
  (Rendering|SetVisibility (Variables|Default|GetStaticMesh) false false))

(event OnComponentEndOverlap(TriggerBox)
  (params (OverlappedComponent :type Primitive%20Component%20Object%20Reference) (OtherActor :type Actor%20Object%20Reference) (OtherComp :type Primitive%20Component%20Object%20Reference) (OtherBodyIndex :type Integer))
  (Utilities|Casting|CastToBP_FPCharacter OtherActor)
  (Widget|RemovefromParent (Variables|Default|GetMessageWidget))
  (Rendering|SetVisibility (Variables|Default|GetStaticMesh) true false))

(event EventBeginPlay)

(event Collision|EventActorBeginOverlap
  (params (OtherActor :type Actor%20Object%20Reference)))

(event EventTick
  (params (DeltaSeconds :type Float%20%28single-precision%29))
  (Utilities|Casting|CastToBP_FPCharacter (Game|Player|GetPlayerPawn 0)
    (:then
      (Transformation|AddActorLocalRotation (Math|Rotator|MakeRotator 0.0 0.0 (* DeltaSeconds 1.2e+02)) false false))
    (:CastFailed
      (bind _messagewidget (Variables|Default|GetMessageWidget)
        (:then
          (Widget|RemovefromParent _messagewidget)
          (Rendering|SetVisibility (Variables|Default|GetStaticMesh) false false))
        (:else)))))

(fn ConstructionScript)