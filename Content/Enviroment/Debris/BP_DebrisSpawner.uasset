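; Debris spawner actor that periodically spawns a random actor class from its Oar array around its own location.
; Tick counts SpawnCooldown down, then spawns at a random X/Y offset, keeping the spawner's height, rotation and scale, and rerolls the cooldown to a few seconds.
; The random index is bounded exclusively by LastIndex, so the final entry is never picked when the array holds several.
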(event EventBeginPlay)

(event Collision|EventActorBeginOverlap
  (params (OtherActor :type Actor%20Object%20Reference)))

(event EventTick
  (params (DeltaSeconds :type Float%20%28single-precision%29))
  (bind _returnvalue (Transformation|GetActorTransform))
  (if (<= (Variables|Default|GetSpawnCooldown) 0.0)
    (Game|SpawnActorfromClass (Utilities|Array|Get(acopy) (Variables|Default|GetOar) (Math|Random|RandomInteger (Utilities|Array|LastIndex (Variables|Default|GetOar)))) (Math|Transform|MakeTransform (Math|Vector|MakeVector (+ (Math|Random|RandomFloatinRange -2e+02 2e+02) (.x (.location _returnvalue))) (+ (Math|Random|RandomFloatinRange -2e+02 2e+02) (.y (.location _returnvalue))) (.z (.location _returnvalue))) (.rotation _returnvalue) (.scale _returnvalue)) "Undefined" 0 0)
    (Variables|Default|SetSpawnCooldown (Math|Random|RandomFloatinRange 1.0 5.0))
    (else
      (Variables|Default|SetSpawnCooldown (- (Variables|Default|GetSpawnCooldown) DeltaSeconds)))))

(fn ConstructionScript)