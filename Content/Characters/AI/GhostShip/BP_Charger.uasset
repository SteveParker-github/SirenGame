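; BP_Charger is an AI-controlled GhostShip enemy that tracks health and dies when it runs out.
; On BeginPlay it links its Charger_Healthbar widget component back to itself and initializes the display.
; AnyDamage reduces Health and refreshes the bar while alive.
; At zero health it calls UnPossess on the AI controller, sets IsDead to ignore further hits, and destroys the actor after a short delay.
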(event EventBeginPlay
  (bind _ascharger_healthbar (Utilities|Casting|CastToCharger_Healthbar (UserInterface|GetWidget (Variables|Default|GetChargerHealthBar))))
  (bind _output_get (Variables|Default|SetChargerHealthWidget _ascharger_healthbar))
  (Variables|/Game/Characters/AI/GhostShip/Charger_Healthbar.Charger_Healthbar_C|SetCharger _output_get self)
  (Default|UpdateHealth _output_get))

(event Game|Damage|EventAnyDamage
  (params (Damage :type Float%20%28single-precision%29) (DamageType :type Damage%20Type%20Object%20Reference) (InstigatedBy :type Controller%20Object%20Reference) (DamageCauser :type Actor%20Object%20Reference))
  (if (not (Variables|Default|GetIsDead))
    (Variables|Default|SetHealth (- (Variables|Default|GetHealth) Damage))
    (Default|UpdateHealth (Variables|Default|GetChargerHealthWidget))
    (if (<= (Variables|Default|GetHealth) 0.0)
      (Pawn|UnPossess (AI|GetAIController (Components|GetOwner)))
      (Variables|Default|SetIsDead true)
      (Utilities|FlowControl|Delay 1.0)
      (Actor|DestroyActor))))

(fn ConstructionScript)