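; Main player controller Blueprint that handles the Zoom input for cycling the minimap's zoom level.
; Each press advances a wrapping index into paired zoom and icon-size arrays, then applies both to the first top-level BP_MinimapHUD widget found, scaling its player icon to match.
; A short delay gate on CanZoom rate-limits presses once a zoom change is applied.
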(event EventBeginPlay)

(event EventTick
  (params (DeltaSeconds :type Float%20%28single-precision%29)))

(event Input|ActionEvents|InputActionZoom
  (params (Key :type Key%20Structure :default "None"))
  (:Pressed
    (if (Variables|Default|GetbCanZoom)
      (bind _result (Math|Integer|IncrementInt (Variables|Default|GetIndex))
        (:%20%20
          (bind _output_get (Variables|Default|SetIndex (Math|Integer|%(Integer) _result (Utilities|Array|Length (Variables|Default|GetZooms)))))
          (Variables|Default|SetNewZoom (Utilities|Array|Get(acopy) (Variables|Default|GetZooms) _output_get))
          (bind _foundwidgets (Widget|GetAllWidgetsOfClass "/Game/UI/MiniMap/BP_MinimapHUD.BP_MinimapHUD_C" true))
          (if (> (Utilities|Array|Length _foundwidgets) 0)
            (Variables|/Game/UI/MiniMap/BP_MinimapWidget.BP_MinimapWidget_C|SetZoom (Variables|/Game/UI/MiniMap/BP_MinimapHUD.BP_MinimapHUD_C|GetBP_MinimapWidget (Utilities|Array|Get(acopy) _foundwidgets)) (Variables|Default|GetNewZoom))
            (bind _output_get_2 (Variables|/Game/UI/MiniMap/BP_MinimapWidget.BP_MinimapWidget_C|SetIconSize (Variables|/Game/UI/MiniMap/BP_MinimapHUD.BP_MinimapHUD_C|GetBP_MinimapWidget (Utilities|Array|Get(acopy) _foundwidgets)) (Utilities|Array|Get(acopy) (Variables|Default|GetIconSize) (Variables|Default|GetIndex))))
            (Widget|Transform|SetRenderScale (Variables|/Game/UI/MiniMap/BP_MinimapHUD.BP_MinimapHUD_C|GetPlayerIcon (Utilities|Array|Get(acopy) _foundwidgets)) _output_get_2)
            (Variables|Default|SetbCanZoom false)
            (Utilities|FlowControl|Delay 0.2)
            (Variables|Default|SetbCanZoom true)))))))

(fn ConstructionScript)